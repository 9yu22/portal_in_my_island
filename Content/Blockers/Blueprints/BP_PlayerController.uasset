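; Player controller for a voxel block game that places and removes blocks in BKChunkBase chunks with the mouse.
; A debug-drawn camera raycast finds the chunk, and the hit point, nudged along its normal, becomes a local block position.
; Right click writes Stone beside the hit face, while left click writes Air to the hit block.
; Removal also spawns a BP_CollapsibleBlock at ModifyVoxel's returned position, set to self-destroy after a delay.
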(event Input|MouseEvents|RightMouseButton
  (params (Key :type Key%20Structure :default "None"))
  (:Pressed
    (bind (_returnvalue _outhit) (CallFunction|Raycast))
    (if _returnvalue
      (bind _asbkchunk_base (Utilities|Casting|CastToBKChunkBase (.HitActor (Collision|BreakHitResult _outhit))))
      (Class|BKChunkBase|ModifyVoxel _asbkchunk_base (Class|KismetMathLibrary|FTruncVector (+ (Class|BKVoxelFunctionLibrary|WorldtoLocalBlockPosition (- (.Location (Collision|BreakHitResult _outhit)) (.Normal (Collision|BreakHitResult _outhit))) (Variables|Default|GetChunkSize)) (.Normal (Collision|BreakHitResult _outhit)))) "Stone"))))

(event Input|MouseEvents|LeftMouseButton
  (params (Key :type Key%20Structure :default "None"))
  (:Pressed
    (bind (_returnvalue _outhit) (CallFunction|Raycast))
    (if _returnvalue
      (bind _asbkchunk_base (Utilities|Casting|CastToBKChunkBase (.HitActor (Collision|BreakHitResult _outhit))))
      (bind _returnvalue_2 (Class|BKChunkBase|ModifyVoxel _asbkchunk_base (Class|BKVoxelFunctionLibrary|WorldtoLocalBlockPosition (- (.Location (Collision|BreakHitResult _outhit)) (.Normal (Collision|BreakHitResult _outhit))) (Variables|Default|GetChunkSize)) "Air"))
      (bind _returnvalue_3 (Game|SpawnActorfromClass "/Game/Blockers/Blueprints/BP_CollapsibleBlock.BP_CollapsibleBlock_C" (Math|Transform|MakeTransform (Math|Conversions|ToVector(Float) _returnvalue_2)) "Undefined" "MultiplyWithRoot" 0 0))
      (bind _returnvalue_4 (AddComponent|AddCollapsibleBlockComponent _returnvalue_3))
      (Class|CollapsibleBlockComponent|DestroyActorwithDelay _returnvalue_4 3.0))))

(fn ConstructionScript)

(fn Raycast
  (bind _playercameramanager (Variables|Default|GetPlayerCameraManager))
  (bind _returnvalue (Camera|GetCameraLocation _playercameramanager))
  (bind (_outhit _returnvalue_2) (Collision|LineTraceByChannel _returnvalue (+ _returnvalue (* (Math|Vector|GetForwardVector (Camera|GetCameraRotation _playercameramanager)) (Variables|Default|GetBlockDistance))) "TraceTypeQuery1" false 0 "ForDuration" true "(R=1.000000,G=0.000000,B=0.000000,A=1.000000)" "(R=0.000000,G=1.000000,B=0.000000,A=1.000000)" 1.0))
  (return _returnvalue_2 _outhit))