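; The HUD class for the Blockers game, which puts the main UI on screen and draws the crosshair.
; On BeginPlay it creates the UIHUD widget for player controller 0 and adds it to the viewport.
; Each DrawHUD call draws the Crosshair texture at a fixed size in the center of the screen using canvas drawing rather than UMG.
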(event EventBeginPlay
  (bind _returnvalue (UserInterface|CreateWidget "/Game/Blockers/Blueprints/UI/GemInventory/UIHUD.UIHUD_C" (Game|GetPlayerController 0)))
  (UserInterface|Viewport|AddtoViewport _returnvalue 0))

(event Collision|EventActorBeginOverlap
  (params (OtherActor :type Actor%20Object%20Reference)))

(event EventTick
  (params (DeltaSeconds :type Float%20%28single-precision%29)))

(event EventDrawHUD
  (params (SizeX :type Integer) (SizeY :type Integer))
  (Canvas|DrawTexture "/Game/BlockGame/Materials/Textures/crosshair.crosshair" (Math|Conversions|ToFloat(Integer) (- (/ SizeX 2) 25)) (Math|Conversions|ToFloat(Integer) (- (/ SizeY 2) 25)) 5e+01 5e+01 0.0 0.0 1.0 1.0 "(R=1.000000,G=1.000000,B=1.000000,A=1.000000)"))

(fn ConstructionScript)