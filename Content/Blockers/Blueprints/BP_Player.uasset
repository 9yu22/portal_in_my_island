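; BP_Player is the player character, with a voxel materialise effect, shop, inventory and camera toggle.
; Tick feeds TL_Transition, mapped across mesh bounds, into the Voxel effect's TransitionLine and refreshes the inventory.
; While Health equals 100, Tick also runs the portal sequence: sounds, material dissolve, movement and input lock, then delayed restore.
; Keys switch first/third person via boom length and owner visibility, toggle ShopUI, and play the shooting montage.
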(event EventTick
  (params (DeltaSeconds :type Float%20%28single-precision%29))
  (bind _mesh (Variables|Character|GetMesh))
  (bind (_origin _boxextent) (Collision|GetComponentBounds _mesh))
  (bind _z (Math|Vector|BreakVector _origin))
  (bind _z_2 (Math|Vector|BreakVector _boxextent))
  ;[0.654 1 0.9621] Start Block Character
  (Utilities|FlowControl|Sequence
    (:then_0
      (Niagara|SetNiagaraVariable(Float) (Variables|Default|GetVoxel) "TransitionLine" (Math|Float|Lerp (- _z _z_2) (+ _z _z_2) (stale _transition))))
    (:then_1
      (if (== (Variables|Default|Gethealth) 1e+02)
        (Audio|PlaySoundatLocation "/Game/Blockers/Blueprints/sound/portalsend.portalsend" "0, 0, 0" "0, 0, 0" 1.0 1.0 0.0 0 0 0 0)
        (Utilities|FlowControl|Sequence
          (:then_0
            (Rendering|SetVisibility (Variables|Character|GetMesh) false false)
            (Input|SetInputModeUIOnly (Game|GetPlayerController 0) 0 "DoNotLock" false)
            (bind _transition (Timeline|TL_Transition Play)
              (:Update
                (Rendering|Material|SetScalarParameterValueonMaterials _mesh "Transition" _transition)
                (Pawn|Components|CharacterMovement|DisableMovement (Variables|Character|GetCharacterMovement))
                (Utilities|FlowControl|Delay 3.5)
                (Utilities|FlowControl|Sequence
                  (:then_0
                    (Rendering|SetVisibility (Variables|Character|GetMesh) true false) ; voxel off, move on
                    (Utilities|FlowControl|DoOnce false :!label _label
                      (:Completed
                        (Audio|PlaySoundatLocation "/Game/Blockers/Blueprints/sound/landisland2.landisland2" "0, 0, 0" "0, 0, 0" 1.0 1.0 0.0 0 0 0 0)
                        (Timeline|TL_Transition Reverse))))
                  (:then_1
                    (Pawn|Components|CharacterMovement|SetMovementMode (Variables|Character|GetCharacterMovement) "MOVE_Walking" 0))
                  (:then_2
                    (Input|SetInputModeGameOnly (Game|GetPlayerController 0) false))))))
          (:then_1
            (goto _label Reset)))))
    (:then_2
      ;;[1 1 1] Inventory
      (Class|BlockersCharacter|UpdateInventory))))

(event Input|ActionEvents|InputActionPrintInventory
  (params (Key :type Key%20Structure :default "None"))
  ;[1 1 1] Second Inventory [keyboard ' I ']
)

(event Input|KeyboardEvents|R
  (params (Key :type Key%20Structure :default "None"))
  (:Pressed
    (Animation|Montage|PlayMontage (Variables|Character|GetMesh) "/Game/Blockers/Blueprints/Character/shootingmontage.shootingmontage" 1.0 0.0 "shoot")))

(event Input|KeyboardEvents|1
  (params (Key :type Key%20Structure :default "None"))
  (bind _returnvalue (Game|GetPlayerController 0))
  (bind _returnvalue_2 (Game|GetPlayerController 0))
  ;[1 1 1] Open Store [1]
  (:Pressed
    (Utilities|FlowControl|FlipFlop
      (:A
        (bind _returnvalue_3 (UserInterface|CreateWidget "/Game/Blockers/Blueprints/UI/Shop/ShopUI.ShopUI_C" _returnvalue_2))
        (Variables|Default|Setshop%20UI _returnvalue_3)
        (UserInterface|Viewport|AddtoViewport _returnvalue_3 0)
        (Variables|/Script/Engine.PlayerController|SetbShowMouseCursor _returnvalue_2 true)
        (Input|SetInputModeGameandUI _returnvalue_2 _returnvalue_3 "DoNotLock" true false))
      (:B
        (Widget|RemovefromParent (Variables|Default|Getshop%20UI))
        (Variables|/Script/Engine.PlayerController|SetbShowMouseCursor _returnvalue false)
        (Input|SetInputModeGameOnly _returnvalue false)))))

(event Input|KeyboardEvents|0
  (params (Key :type Key%20Structure :default "None"))
  (bind _staticmesh (Variables|Default|GetStaticMesh))
  (bind _mesh (Variables|Character|GetMesh))
  (bind _cameraboom (Variables|Default|GetCameraBoom))
  (bind _cameraboom_2 (Variables|Default|GetCameraBoom))
  (:Pressed
    (bind _output_get (Variables|Default|SetFirstPersonCamera (not (Variables|Default|GetFirstPersonCamera))))
    (if _output_get
      (Variables|/Script/Engine.SpringArmComponent|SetTargetArmLength _cameraboom_2 0.0)
      (Transformation|SetRelativeLocation _cameraboom_2 "0.000000,0.000000,50.000000" false false)
      (Class|PrimitiveComponent|SetOwnerNoSee _mesh true)
      (Class|PrimitiveComponent|SetOwnerNoSee _staticmesh true)
      (else
        (Variables|/Script/Engine.SpringArmComponent|SetTargetArmLength _cameraboom 4e+02)
        (Transformation|SetRelativeLocation _cameraboom "0.000000,0.000000,40.000000" false false)
        (Class|PrimitiveComponent|SetOwnerNoSee _mesh false)
        (Class|PrimitiveComponent|SetOwnerNoSee _staticmesh false)))))

(fn ConstructionScript)