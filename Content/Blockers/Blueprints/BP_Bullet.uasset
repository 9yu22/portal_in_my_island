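; Bullet actor that knocks a block out of voxel chunk terrain on impact and leaves a bomb at the hit point.
; Tick waits for a hit on a BKChunkBase, then sets that voxel to Air using the player controller's chunk size.
; It spawns a stone collapsible block in the voxel's place with delayed destruction, spawns BP_Bomb, then destroys itself.
; Nothing in these graphs sets the hit state.
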(event EventBeginPlay)

(event Collision|EventActorBeginOverlap
  (params (OtherActor :type Actor%20Object%20Reference)))

(event EventTick
  (params (DeltaSeconds :type Float%20%28single-precision%29))
  (bind _hitresult (Variables|Default|GetHitResult))
  (bind (_bblockinghit _binitialoverlap _time _distance _location _impactpoint _normal _impactnormal _physmat _hitactor) (Collision|BreakHitResult _hitresult))
  (bind _returnvalue (- _location _normal))
  (if (Variables|Default|GetbHit)
    (bind _asbp_player_controller (Utilities|Casting|CastToBP_PlayerController (Pawn|GetController (Game|Player|GetPlayerPawn 0))))
    (bind _asbkchunk_base (Utilities|Casting|CastToBKChunkBase _hitactor))
    (Class|BKChunkBase|ModifyVoxel _asbkchunk_base (Class|BKVoxelFunctionLibrary|WorldtoLocalBlockPosition _returnvalue _normal (Variables|/Game/Blockers/Blueprints/Game/BP_PlayerController.BP_PlayerController_C|GetChunkSize _asbp_player_controller)) "Air")
    (bind _returnvalue_2 (Game|SpawnActorfromClass "/Game/Blockers/Blueprints/BP_CollapsibleBlock_Stone.BP_CollapsibleBlock_Stone_C" (Math|Transform|MakeTransform (Math|Conversions|ToVector(Float) (Class|BKVoxelFunctionLibrary|GetBlockWorldPostion _returnvalue _normal (Variables|/Game/Blockers/Blueprints/Game/BP_PlayerController.BP_PlayerController_C|GetChunkSize _asbp_player_controller)))) "Undefined" "MultiplyWithRoot" 0 0))
    (bind _returnvalue_3 (AddComponent|AddCollapsibleBlockComponent _returnvalue_2))
    (Class|CollapsibleBlockComponent|DestroyActorwithDelay _returnvalue_3 3.0)
    (Game|SpawnActorfromClass "/Game/Blockers/Blueprints/BP_Bomb.BP_Bomb_C" (Math|Transform|MakeTransform _impactpoint) "Undefined" "MultiplyWithRoot" 0 0)
    (Actor|DestroyActor)))

(fn ConstructionScript)